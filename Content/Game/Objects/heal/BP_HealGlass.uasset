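; BP_HealGlass is a healing pickup that restores Life to Bp_Erika when she overlaps its Box.
; Each overlap spends a HealCount charge, even at full Life; a heal destroys the glass and spawns a replacement at a random XY position.
; With no charges left, the overlap refills HealCount after a delay.
; A similar BP_Maw branch with a larger heal and no refill is disconnected and never runs.
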(event OnComponentBeginOverlap(Box)
  (params (OverlappedComponent :type Primitive%20Component%20Object%20Reference) (OtherActor :type Actor%20Object%20Reference) (OtherComp :type Primitive%20Component%20Object%20Reference) (OtherBodyIndex :type Integer) (bFromSweep :type Boolean) (SweepResult :type Hit%20Result%20Structure%20%28by%20ref%29))
  (bind _asbp_erika (Utilities|Casting|CastToBp_Erika OtherActor))
  (bind _output_get (Variables|Default|SetBp%20Erika _asbp_erika))
  (if (> (Variables|/Game/Game/Characters/Humans/Erika/Bp_Erika.Bp_Erika_C|GetHeal%20Count _output_get) 0.0)
    (Variables|/Game/Game/Characters/Humans/Erika/Bp_Erika.Bp_Erika_C|SetHeal%20Count (Variables|Default|GetBp%20Erika) (- (Variables|/Game/Game/Characters/Humans/Erika/Bp_Erika.Bp_Erika_C|GetHeal%20Count _output_get) 1.0))
    (if (< (Variables|/Game/Game/Characters/Humans/Erika/Bp_Erika.Bp_Erika_C|GetLife _output_get) (Variables|/Game/Game/Characters/Humans/Erika/Bp_Erika.Bp_Erika_C|GetMax%20Life _output_get))
      (bind _output_get_2 (Variables|/Game/Game/Characters/Humans/Erika/Bp_Erika.Bp_Erika_C|SetLife (Variables|Default|GetBp%20Erika) (+ (Variables|/Game/Game/Characters/Humans/Erika/Bp_Erika.Bp_Erika_C|GetLife (Variables|Default|GetBp%20Erika)) 1e+01)))
      (Development|PrintString (Utilities|String|ToString(Float) _output_get_2))
      (Actor|DestroyActor)
      (Game|SpawnActorfromClass "BP_HealGlass_C" (Math|Transform|MakeTransform (Math|Vector|MakeVector (Math|Conversions|ToFloat(Integer) (Math|Random|RandomIntegerinRange 1 500)) (Math|Conversions|ToFloat(Integer) (Math|Random|RandomIntegerinRange 1 500)) 1.9e+02)) "Undefined" 0 0)
      (else
        (Development|PrintString "pas de soins chacal")))
    (else
      (Utilities|FlowControl|Delay 15.0)
      (Variables|/Game/Game/Characters/Humans/Erika/Bp_Erika.Bp_Erika_C|SetHeal%20Count (Variables|Default|GetBp%20Erika) 3.0)
      (Development|PrintString "a nouveau 3 soins"))))

(fn ConstructionScript)