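; Player mage character Wiezzorek, with fireball and lightning strike attacks, sprint, healing and a save/load menu.
; Attacks lock movement, spawn spell actors after a timed wind-up, and use delays for cleanup and cooldowns.
; Heal charges restore Life, are replenished by sphere-trace pickup of BP_HealGlass, and update a HUD counter.
; Damage drains Life toward death and Game Over; the save menu casts the player to Bp_Erika, not this class.
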(event EventBeginPlay
  (bind _returnvalue (UserInterface|CreateWidget "/Game/Game/UI/HUD/Spell_HUD.Spell_HUD_C"))
  (UserInterface|Viewport|AddtoViewport _returnvalue 0)
  (bind _returnvalue_2 (UserInterface|CreateWidget "/Game/Game/UI/HUD/HealCount_HUD.HealCount_HUD_C" (Game|GetPlayerController 0)))
  (Variables|Default|SetHeal%20Count%20HUD _returnvalue_2)
  (bind _asbp_wiezzorek (Utilities|Casting|CastToBP_wiezzorek (Game|GetPlayerCharacter 0)))
  (Rendering|Components|TextRender|SetText (Variables|/Game/Game/UI/HUD/HealCount_HUD.HealCount_HUD_C|GetHealCount _returnvalue_2) (Utilities|Text|ToText(String) (Utilities|String|Append (Utilities|String|ToString(Float) (Variables|BP_wiezzorek_C|GetHeal%20Count _asbp_wiezzorek)) " Heals")))
  (UserInterface|Viewport|AddtoViewport _returnvalue_2 0))

(event Game|Damage|EventAnyDamage
  (params (Damage :type Float%20%28single-precision%29) (DamageType :type Damage%20Type%20Object%20Reference) (InstigatedBy :type Controller%20Object%20Reference) (DamageCauser :type Actor%20Object%20Reference))
  (if (> (Variables|Default|GetLife) 0.0)
    (bind _output_get (Variables|Default|SetLife (- (Variables|Default|GetLife) Damage)))
    (Development|PrintString (Utilities|String|ToString(Float) _output_get))
    (if (== (Variables|Default|GetLife) 0.0)
      (Components|Animation|PlayAnimation (Variables|Character|GetMesh) "/Game/Game/Animations/Mage/Wiezzorek/Dying.Dying" false)
      (Input|DisableInput (Game|GetPlayerCharacter 0) 0)
      (bind _returnvalue (UserInterface|CreateWidget "/Game/Game/UI/HUD/Gameover_HUD.GameOver_HUD_C" :!label _label))
      (UserInterface|Viewport|AddtoViewport _returnvalue 0))
    (else
      (Components|Animation|PlayAnimation (Variables|Character|GetMesh) "/Game/Game/Animations/Mage/Wiezzorek/Dying.Dying" false)
      (Input|DisableInput (Game|GetPlayerCharacter 0) 0)
      (goto _label))))

(event Input|ActionEvents|InputActionSprint
  (params (Key :type Key%20Structure :default "None"))
  (bind _charactermovement (Variables|Character|GetCharacterMovement))
  ;[0 1 0] Sprint
  (:Pressed
    (Variables|/Script/Engine.CharacterMovementComponent|SetMaxWalkSpeed _charactermovement 3e+02))
  (:Released
    (Variables|/Script/Engine.CharacterMovementComponent|SetMaxWalkSpeed _charactermovement 1.5e+02)))

(event Input|ActionEvents|InputActionattackPrimary
  (params (Key :type Key%20Structure :default "None"))
  (bind _camera (Variables|Default|GetCamera))
  (bind _mesh (Variables|Character|GetMesh))
  (bind _charactermovement (Variables|Character|GetCharacterMovement))
  (bind _charactermovement_2 (Variables|Character|GetCharacterMovement))
  (bind _returnvalue (Transformation|GetWorldRotation _camera))
  (bind (_roll _pitch _yaw) (Math|Rotator|BreakRotator _returnvalue))
  (:Pressed
    (if (not (Variables|Default|Getis_principal_cooldown))
      (Variables|Default|Setis_principal_cooldown true)
      (Variables|/Script/Engine.CharacterMovementComponent|SetMaxWalkSpeed _charactermovement 0.0)
      (Variables|/Script/Engine.CharacterMovementComponent|SetJumpZVelocity _charactermovement 0.0)
      (Variables|Default|Setis_Attacking true)
      (Utilities|FlowControl|Delay 1.9)
      (bind _returnvalue_2 (Game|SpawnActorfromClass "/Game/Game/Objects/fireball.fireball_C" (Math|Transform|MakeTransform (+ (Transformation|GetWorldLocation _mesh) (* (Math|Vector|GetRightVector _mesh) 1.5e+02) "0,0.000000,120.000000") (Math|Rotator|MakeRotator 0.0 _pitch _yaw)) "AlwaysSpawn" 0 0))
      (AddComponent|AddProjectileMovementComponent _returnvalue_2)
      (Variables|Default|Setis_Attacking false)
      (Variables|/Script/Engine.CharacterMovementComponent|SetMaxWalkSpeed _charactermovement_2 1.5e+02)
      (Variables|/Script/Engine.CharacterMovementComponent|SetJumpZVelocity _charactermovement_2 4e+02)
      (Utilities|FlowControl|Delay 2.0)
      (Actor|DestroyActor _returnvalue_2)
      (Utilities|FlowControl|Delay 1.0)
      (Variables|Default|Setis_principal_cooldown false))))

(event Input|ActionEvents|InputActionInteract
  (params (Key :type Key%20Structure :default "None"))
  (bind _camera (Variables|Default|GetCamera))
  (bind _camera_2 (Variables|Default|GetCamera))
  ;[1 1 0] Interact to objects
  (:Pressed
    (bind _outhit (Collision|SphereTraceByChannel (+ (Transformation|GetWorldLocation _camera) (* (Math|Vector|GetForwardVector _camera) 3e+02)) (+ (Transformation|GetWorldLocation _camera_2) (* (Math|Vector|GetForwardVector _camera_2) 4e+02)) 2e+01 "TraceTypeQuery1" false 0 "None"))
    (Utilities|Casting|CastToBP_chest (.hitactor _outhit)
      (:CastFailed
        (Utilities|Casting|CastToBP_HealGlass (.hitactor _outhit))
        (Variables|Default|SetisInteracting true)
        (Utilities|FlowControl|Delay 2.4)
        (bind _output_get (Variables|Default|SetHeal%20Count (+ (Variables|Default|GetHeal%20Count) 1.0)))
        (Rendering|Components|TextRender|SetText (Variables|/Game/Game/UI/HUD/HealCount_HUD.HealCount_HUD_C|GetHealCount (Variables|Default|GetHeal%20Count%20HUD)) (Utilities|Text|ToText(String) (Utilities|String|Append (Utilities|String|ToString(Float) _output_get) " Heals")))
        (Actor|DestroyActor (.hitactor _outhit))
        (Variables|Default|SetisInteracting false)))))

(event Input|ActionEvents|InputActionAttackSecondary
  (params (Key :type Key%20Structure :default "None"))
  (bind _mesh (Variables|Character|GetMesh))
  (bind _camera (Variables|Default|GetCamera))
  (bind _charactermovement (Variables|Character|GetCharacterMovement))
  (bind _charactermovement_2 (Variables|Character|GetCharacterMovement))
  (bind _returnvalue (Transformation|GetWorldRotation _camera))
  (bind (_roll _pitch _yaw) (Math|Rotator|BreakRotator _returnvalue))
  (:Pressed
    (if (not (Variables|Default|Getis_secondary_cooldown))
      (Variables|Default|Setis_secondary_cooldown true)
      (Variables|/Script/Engine.CharacterMovementComponent|SetMaxWalkSpeed _charactermovement 0.0)
      (Variables|/Script/Engine.CharacterMovementComponent|SetJumpZVelocity _charactermovement 0.0)
      (Variables|Default|Setis_Attacking true)
      (Utilities|FlowControl|Delay 1.9)
      (bind _returnvalue_2 (Game|SpawnActorfromClass "/Game/Game/Objects/LightningStrike.LightningStrike_C" (Math|Transform|MakeTransform (+ (Transformation|GetWorldLocation _mesh) (* (Math|Vector|GetRightVector _mesh) 1.5e+02) "50.000000,0.000000,120.000000") (Math|Rotator|MakeRotator _roll 0.0 _yaw)) "AlwaysSpawn" 0 0))
      (Variables|Default|Setis_Attacking false)
      (Utilities|FlowControl|Delay 3.0)
      (Actor|DestroyActor _returnvalue_2)
      (Variables|/Script/Engine.CharacterMovementComponent|SetMaxWalkSpeed _charactermovement_2 1.5e+02)
      (Variables|/Script/Engine.CharacterMovementComponent|SetJumpZVelocity _charactermovement_2 4e+02)
      (Utilities|FlowControl|Delay 0.5)
      (Variables|Default|Setis_secondary_cooldown false))))

(event Input|ActionEvents|InputActionHeal
  (params (Key :type Key%20Structure :default "None"))
  (bind _returnvalue (Game|GetPlayerCharacter 0))
  (:Pressed
    (bind _returnvalue_2 (Game|SpawnActorfromClass "/Game/Game/Objects/HealEffect.HealEffect_C" (Math|Transform|MakeTransform (- (Transformation|GetWorldLocation (Variables|/Script/Engine.Character|GetCapsuleComponent _returnvalue)) "0,5.000000, 0")) "Undefined" _returnvalue _returnvalue))
    (if (> (Variables|Default|GetHeal%20Count) 0.0)
      (Variables|Default|SetLife (+ (Variables|Default|GetLife) 1e+01))
      (bind _output_get (Variables|Default|SetHeal%20Count (- (Variables|Default|GetHeal%20Count) 1.0)))
      (Rendering|Components|TextRender|SetText (Variables|/Game/Game/UI/HUD/HealCount_HUD.HealCount_HUD_C|GetHealCount (Variables|Default|GetHeal%20Count%20HUD)) (Utilities|Text|ToText(String) (Utilities|String|Append (Utilities|String|ToString(Float) _output_get) " Heals")))
      (Utilities|FlowControl|Delay 1.0)
      (Actor|DestroyActor _returnvalue_2))))

(event Input|ActionEvents|InputActionSaveMenu
  (params (Key :type Key%20Structure :default "None"))
  (bind _returnvalue (Game|GetPlayerCharacter 0))
  (:Pressed
    (Utilities|FlowControl|FlipFlop
      (:A
        (Input|DisableInput _returnvalue (Game|GetPlayerController 0))
        (Variables|Default|Setis_In_Pause true)
        (bind _returnvalue_2 (UserInterface|CreateWidget "/Game/Game/UI/HUD/Save_and_Load_HUD.Save_and_Load_HUD_C"))
        (bind _asbp_erika (Utilities|Casting|CastToBp_Erika _returnvalue))
        (Variables|/Game/Game/UI/HUD/Save_and_Load_HUD.Save_and_Load_HUD_C|SetPlayerCharacter _returnvalue_2 _asbp_erika)
        (UserInterface|Viewport|AddtoViewport _returnvalue_2 0))
      (:B
        (Widget|RemovefromParent _returnvalue_2)))))

(fn ConstructionScript
  (|CallParentFunction))