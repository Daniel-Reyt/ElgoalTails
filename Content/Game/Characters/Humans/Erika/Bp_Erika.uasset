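; Erika is a playable human character with melee attack, block, sprint and damage-driven death.
; BeginPlay attaches a Dragon_Blade and Shield to hand sockets and adds them to Inventory.
; Inputs set attack/block flags and adjust walk speed and jump velocity, restoring them after delays; Interact sphere-traces for BP_chest but takes no action after the cast.
; Damage reduces Life; death plays Dying, disables input and shows GameOver_HUD.
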(event EventBeginPlay
  (bind _mesh (Variables|Character|GetMesh))
  ;[0 1 0] Attach SHield And Weapon
  (bind _returnvalue (Game|SpawnActorfromClass "/Game/Game/Weapons/Erika/Dragon_Blade.Dragon_Blade_C" (Transformation|GetSocketTransform (Variables|Character|GetMesh) "Weapon_Hold" "RTS_World") "Undefined" 0 0))
  (Transformation|AttachComponentToComponent _returnvalue _mesh "Weapon_Hold" "SnapToTarget" "SnapToTarget" "SnapToTarget" true)
  (Utilities|Array|Add (Variables|Default|GetInventory) _returnvalue)
  (bind _returnvalue_2 (Game|SpawnActorfromClass "/Game/Game/Weapons/Erika/Shield.Shield_C" (Transformation|GetSocketTransform _mesh "Shield_Hold" "RTS_World") "Undefined" 0 0))
  (Transformation|AttachComponentToComponent _returnvalue_2 (Variables|Character|GetMesh) "Shield_Hold" "SnapToTarget" "SnapToTarget" "SnapToTarget" true)
  (Utilities|Array|Add (Variables|Default|GetInventory) _returnvalue_2))

(event Game|Damage|EventAnyDamage
  (params (Damage :type Float%20%28single-precision%29) (DamageType :type Damage%20Type%20Object%20Reference) (InstigatedBy :type Controller%20Object%20Reference) (DamageCauser :type Actor%20Object%20Reference))
  (if (> (Variables|Default|GetLife) 0.0)
    (Variables|Default|SetLife (- (Variables|Default|GetLife) Damage))
    (Development|PrintString (Utilities|String|ToString(Float) (Variables|Default|GetLife)))
    (if (== (Variables|Default|GetLife) 0.0)
      (Components|Animation|PlayAnimation (Variables|Character|GetMesh) "/Game/Game/Animations/Humans/Erika/Dying.Dying" false)
      (Input|DisableInput (Game|GetPlayerCharacter 0) 0)
      (bind _returnvalue (UserInterface|CreateWidget "/Game/Game/UI/HUD/Gameover_HUD.GameOver_HUD_C" :!label _label))
      (UserInterface|Viewport|AddtoViewport _returnvalue 0))
    (else
      (Components|Animation|PlayAnimation (Variables|Character|GetMesh) "/Game/Game/Animations/Humans/Erika/Dying.Dying" false)
      (Input|DisableInput (Game|GetPlayerCharacter 0) 0)
      (goto _label))))

(event Input|ActionEvents|InputActionSprint
  (params (Key :type Key%20Structure :default "None"))
  (bind _charactermovement (Variables|Character|GetCharacterMovement))
  ;[0 1 0] Sprint
  (:Pressed
    (Variables|/Script/Engine.CharacterMovementComponent|SetMaxWalkSpeed _charactermovement 3e+02))
  (:Released
    (Variables|/Script/Engine.CharacterMovementComponent|SetMaxWalkSpeed _charactermovement 1.5e+02)))

(event Input|ActionEvents|InputActionattackPrimary
  (params (Key :type Key%20Structure :default "None"))
  (bind _charactermovement (Variables|Character|GetCharacterMovement))
  (bind _charactermovement_2 (Variables|Character|GetCharacterMovement))
  ;[0 1 0] Attack
  (:Pressed
    (Variables|/Script/Engine.CharacterMovementComponent|SetMaxWalkSpeed _charactermovement 0.0)
    (Variables|/Script/Engine.CharacterMovementComponent|SetJumpZVelocity _charactermovement 0.0)
    (Variables|Default|Setis_Attacking true)
    (Utilities|FlowControl|Delay 1.08)
    (Variables|Default|Setis_Attacking false)
    (Variables|/Script/Engine.CharacterMovementComponent|SetMaxWalkSpeed _charactermovement_2 1.5e+02)
    (Variables|/Script/Engine.CharacterMovementComponent|SetJumpZVelocity _charactermovement_2 4e+02)))

(event Input|ActionEvents|InputActionInteract
  (params (Key :type Key%20Structure :default "None"))
  (bind _camera (Variables|Default|GetCamera))
  (bind _camera_2 (Variables|Default|GetCamera))
  ;[1 1 0] Interact to objects
  (:Pressed
    (bind _outhit (Collision|SphereTraceByChannel (+ (Transformation|GetWorldLocation _camera) (* (Math|Vector|GetForwardVector _camera) 3e+02)) (+ (Transformation|GetWorldLocation _camera_2) (* (Math|Vector|GetForwardVector _camera_2) 4e+02)) 2e+01 "TraceTypeQuery1" false 0 "Persistent"))
    (Utilities|Casting|CastToBP_chest (.hitactor _outhit))))

(event Input|ActionEvents|InputActionAttackSecondary
  (params (Key :type Key%20Structure :default "None"))
  (bind _charactermovement (Variables|Character|GetCharacterMovement))
  (bind _charactermovement_2 (Variables|Character|GetCharacterMovement))
  ;[0 1 0] Block
  (:Pressed
    (Variables|/Script/Engine.CharacterMovementComponent|SetMaxWalkSpeed _charactermovement_2 0.0)
    (Variables|/Script/Engine.CharacterMovementComponent|SetJumpZVelocity _charactermovement_2 0.0)
    (Variables|Default|Setis_blocking true))
  (:Released
    (Utilities|FlowControl|Delay 0.7)
    (Variables|Default|Setis_blocking false)
    (Variables|/Script/Engine.CharacterMovementComponent|SetMaxWalkSpeed _charactermovement 1.5e+02)
    (Variables|/Script/Engine.CharacterMovementComponent|SetJumpZVelocity _charactermovement 4e+02)))

(fn ConstructionScript
  (|CallParentFunction))

(fn ReturnPlayerHasMove
  (return false))