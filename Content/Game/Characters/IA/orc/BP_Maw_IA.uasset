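; BP_Maw_IA is an orc AI character Blueprint that handles taking damage and dying.
; AnyDamage subtracts damage from Life and prints the remaining value to screen.
; When Life runs out, it zeroes walk speed, plays the Dying animation, destroys its Axe, then removes itself after a short delay.
; Hits received after death only keep walk speed at zero.
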(event Game|Damage|EventAnyDamage
  (params (Damage :type Float%20%28single-precision%29) (DamageType :type Damage%20Type%20Object%20Reference) (InstigatedBy :type Controller%20Object%20Reference) (DamageCauser :type Actor%20Object%20Reference))
  (if (> (Variables|Default|GetLife) 0.0)
    (Variables|Default|SetLife (- (Variables|Default|GetLife) Damage))
    (Development|PrintString (Utilities|String|ToString(Float) (Variables|Default|GetLife)))
    (if (<= (Variables|Default|GetLife) 0.0)
      (Variables|/Script/Engine.CharacterMovementComponent|SetMaxWalkSpeed (Variables|Character|GetCharacterMovement) 0.0)
      (Components|Animation|PlayAnimation (Variables|Character|GetMesh) "/Game/Game/Animations/Orcs/Maw/Dying.Dying" false)
      (Actor|DestroyActor (Variables|Default|GetAxe))
      (Utilities|FlowControl|Delay 4.5)
      (Actor|DestroyActor))
    (else
      (Variables|/Script/Engine.CharacterMovementComponent|SetMaxWalkSpeed (Variables|Character|GetCharacterMovement) 0.0))))

(fn ConstructionScript
  (|CallParentFunction))